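; BP_Block is a breakable block actor that loses health each time a BP_Ball hits it and destroys itself at zero.
; On BeginPlay it creates a dynamic instance of M_Castom on its static mesh and records its starting health.
; Each ball hit sets the material's Color parameter from the fraction of health lost, shifting it from black toward red as damage builds.
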(event `self.ReceiveBeginPlay`
  (bind _returnvalue (`PrimitiveComponent.CreateDynamicMaterialInstance` (`self.StaticMesh`) 0 "/Game/Materials/M_Castom.M_Castom" "None"))
  (set `self.DynamicMaterial` _returnvalue)
  (set `self.StartHealth` (`self.Health`)))

(event `self.ReceiveHit`
  (params (MyComp :type "PrimitiveComponent Object Reference") (Other :type "Actor Object Reference") (OtherComp :type "PrimitiveComponent Object Reference") (bSelfMoved :type Boolean) (HitLocation :type "Vector Structure") (HitNormal :type "Vector Structure") (NormalImpulse :type "Vector Structure") (Hit :type "HitResult Structure (by ref)"))
  (cast `/Game/BP_Ball` Other)
  (bind _output_get (set `self.Health` (- (`self.Health`) 1)))
  (`MaterialInstanceDynamic.SetVectorParameterValue` (`self.DynamicMaterial`) "Color" (make `LinearColor` (/ (`KismetMathLibrary.Conv_IntToDouble` (- (`self.StartHealth`) (`self.Health`))) (`KismetMathLibrary.Conv_IntToDouble` (`self.StartHealth`))) 0.0 0.0 1.0))
  (if (== _output_get 0)
    (`self.K2_DestroyActor`)))

(fn `UserConstructionScript`)