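; BP_Pawn is the player pawn, which slides sideways on the Move axis and spawns the ball in play.
; On BeginPlay it spawns a half-scale BP_Ball at its Sphere component and binds the ball's OnDead event to RespawnBall.
; RespawnBall loops back into the same spawn logic unless BP_GameMode's Health is zero.
; Movement uses fixed swept Y offsets per input call, without delta-time scaling.
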(event `self.ReceiveBeginPlay`
  (bind _returnvalue (`|SpawnActorFromClass` "/Game/BP_Ball.BP_Ball_C" (`KismetMathLibrary.MakeTransform` (`SceneComponent.K2_GetComponentLocation` (`self.Sphere`)) (struct) (0.5 0.5 0.5)) "Undefined" "OverrideRootScale" null null :!label _label))
  (add `/Game/BP_Ball.OnDead` _returnvalue (delegate `RespawnBall`)))

(event `RespawnBall`
  (bind _asbp_game_mode (cast `/Game/BP_GameMode` (`GameplayStatics.GetGameMode`)))
  (if (not (== (`/Game/BP_GameMode.Health` _asbp_game_mode) 0))
    (goto _label)))

(event `self.ReceiveTick`
  (params (DeltaSeconds :type "Float (single-precision)")))

(event `InputAxis|Move`
  (params (AxisValue :type "Float (single-precision)"))
  (if (> AxisValue 0.0)
    (`self.K2_AddActorWorldOffset` (0.0 15.0 0.0) true)
    (elif (< AxisValue 0.0)
      (`self.K2_AddActorWorldOffset` (0.0 -15.0 0.0) true))))

(fn `UserConstructionScript`)