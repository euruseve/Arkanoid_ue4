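; BP_BlockIncreaseSpeed is a breakable block that speeds up the ball that hits it.
; On a hit from BP_Ball it doubles the ball's Speed, unless the result would exceed three times DefaultSpeed.
; It then always calls the ball's TimerForResetSpeed, runs CheckBlockCount and destroys itself.
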(event `self.ReceiveHit`
  (params (MyComp :type "PrimitiveComponent Object Reference") (Other :type "Actor Object Reference") (OtherComp :type "PrimitiveComponent Object Reference") (bSelfMoved :type Boolean) (HitLocation :type "Vector Structure") (HitNormal :type "Vector Structure") (NormalImpulse :type "Vector Structure") (Hit :type "HitResult Structure (by ref)"))
  (bind _asbp_ball (cast `/Game/Blueprints/BP_Ball` Other))
  (bind _returnvalue (* (`/Game/Blueprints/BP_Ball.Speed` _asbp_ball) 2.0))
  (if (not (> _returnvalue (* (`/Game/Blueprints/BP_Ball.DefaultSpeed` _asbp_ball) 3.0)))
    (set `/Game/Blueprints/BP_Ball.Speed` _returnvalue _asbp_ball))
  (`/Game/Blueprints/BP_Ball.TimerForResetSpeed` _asbp_ball)
  (`self.CheckBlockCount`)
  (`self.K2_DestroyActor`))

(fn `UserConstructionScript`)