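; Ball actor that travels in a straight line, bounces off surfaces and costs the player health when lost.
; Tick applies a swept offset of Direction times Speed, unscaled by delta time, and reflects Direction on blocking hits.
; Overlapping a KillZVolume lowers health through BP_GameMode, calls CallOnDead and destroys the ball.
; TimerForResetSpeed restores the Speed saved at BeginPlay after a short delay.
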(event `self.ReceiveBeginPlay`
  (set `self.DefaultSpeed` (`self.Speed`)))

(event `self.ReceiveActorBeginOverlap`
  (params (OtherActor :type "Actor Object Reference"))
  (cast `KillZVolume` OtherActor)
  (bind _asbp_game_mode (cast `/Game/Blueprints/BP_GameMode` (`GameplayStatics.GetGameMode`)))
  (`/Game/Blueprints/BP_GameMode.ChangeHealth` _asbp_game_mode -1)
  (`self.OnDead`)
  (`self.K2_DestroyActor`))

(event `self.ReceiveTick`
  (params (DeltaSeconds :type "Float (single-precision)"))
  (bind _sweephitresult (`self.K2_AddActorWorldOffset` (* (`self.Direction`) (`self.Speed`)) true))
  (bind (_bblockinghit _binitialoverlap _time _distance _location _impactpoint _normal) (`GameplayStatics.BreakHitResult` _sweephitresult))
  (if _bblockinghit
    (set `self.Direction` (`KismetMathLibrary.GetReflectionVector` (`self.Direction`) _normal))))

(event `TimerForResetSpeed`
  (`KismetSystemLibrary.K2_SetTimerDelegate` (delegate `ResetSpeed`) 2.0))

(event `ResetSpeed`
  (set `self.Speed` (`self.DefaultSpeed`)))

(fn `UserConstructionScript`)