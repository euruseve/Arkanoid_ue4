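; BP_GameMode is a game mode that tracks Health and manages the health bar and game-over screens.
; On BeginPlay it creates a WBP_HealthBar widget, stores it and adds it to the viewport.
; ChangeHealth adds a delta to Health without clamping, refreshes the health bar, and shows WBP_GameOverMenu only when Health equals exactly zero.
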(event `self.ReceiveBeginPlay`
  (bind _returnvalue (`|CreateWidget` "/Game/Widgets/WBP_HealthBar.WBP_HealthBar_C"))
  (bind _output_get (set `self.WidgetHealthBar` _returnvalue))
  (`UserWidget.AddToViewport` _output_get 0))

(fn `ChangeHealth`
  (params (Delta :type Integer))
  (bind _output_get (set `self.Health` (+ (`self.Health`) Delta)))
  (`/Game/Widgets/WBP_HealthBar.ChangeHealthCount` (`self.WidgetHealthBar`))
  (if (== _output_get 0)
    (bind _returnvalue (`|CreateWidget` "/Game/Widgets/WBP_GameOverMenu.WBP_GameOverMenu_C"))
    (`UserWidget.AddToViewport` _returnvalue 0)))

(fn `UserConstructionScript`)